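; Custom Game Instance that holds player, companion dog and level progress data, presumably to carry it between levels.
; Init events register references to the player, dog AI and progress manager, with only the first player registration automatically snapshotting its inventory.
; Update events copy inventory, dog mission data and current level into the instance, individually or through UpdateAllInformation.
; Matching LoadData events write the stored values back onto those objects.
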(event Custom|InitPlayerRef
  (params (Player%20Character%20Ref :type BP%20First%20Person%20Character%20Object%20Reference))
  ;[0.15 0.15 0.15 0.5] Collecting References
  (Variables|Default|SetPlayer%20Character Player%20Character%20Ref)
  (Utilities|FlowControl|Sequence
    (:then_0
      (Utilities|FlowControl|DoOnce false
        (:Completed
          (CallFunction|UpdatePlayerInformation))))))

(event Custom|UpdateLevelProgress
  ;[0.15 0.15 0.15 0.5] Updating Information
  (Variables|Default|SetCurrent%20Level (Variables|/Game/Blueprints/Data/BP_ProgressManager.BP_ProgressManager_C|GetCurrentLevel (Variables|Default|GetProgress%20Manager))))

(event Custom|LoadDataDog
  (bind _dog_ai (Variables|Default|GetDog%20AI))
  (Variables|/Game/Blueprints/BP_Dog.BP_Dog_C|SetInteger _dog_ai (Variables|Default|GetInteger))
  (Variables|/Game/Blueprints/AIC_Companion.AIC_Companion_C|SetMissonObjects (Variables|/Game/Blueprints/BP_Dog.BP_Dog_C|GetAs%20AIC%20Companion _dog_ai) (Variables|Default|GetMisson%20Objects)))

(event Custom|LoadDataLevel
  (Variables|/Game/Blueprints/Data/BP_ProgressManager.BP_ProgressManager_C|SetCurrentLevel (Variables|Default|GetProgress%20Manager) (Variables|Default|GetCurrent%20Level)))

(event Custom|InitDogRef
  (params (Dog%20Ref :type BP%20Dog%20Object%20Reference))
  ;[0.15 0.15 0.15 0.5] Collecting References
  (Variables|Default|SetDog%20AI Dog%20Ref))

(event Custom|LoadDataPlayer
  (Variables|/Game/FirstPerson/Blueprints/BP_FirstPersonCharacter.BP_FirstPersonCharacter_C|SetTempInventory (Variables|Default|GetPlayer%20Character) (Variables|PlayerData|GetTemp%20Inventory)))

(event Custom|UpdatePlayerInformation
  ;[0.15 0.15 0.15 0.5] Updating Information
  (Variables|PlayerData|SetTemp%20Inventory (Variables|/Game/FirstPerson/Blueprints/BP_FirstPersonCharacter.BP_FirstPersonCharacter_C|GetTempInventory (Variables|Default|GetPlayer%20Character))))

(event Custom|UpdateAllInformation
  ;[0.15 0.0625 0.0625 0.5] Information Update HUB
  (CallFunction|UpdatePlayerInformation)
  (CallFunction|UpdateDogInformation)
  (CallFunction|UpdateLevelProgress))

(event Custom|InitProgressManager
  (params (Progress%20Manager :type BP%20Progress%20Manager%20Object%20Reference))
  ;[0.15 0.15 0.15 0.5] Collecting References
  (Variables|Default|SetProgress%20Manager Progress%20Manager))

(event Custom|UpdateDogInformation
  (bind _dog_ai (Variables|Default|GetDog%20AI))
  ;[0.15 0.15 0.15 0.5] Updating Information
  (Variables|Default|SetInteger (Variables|/Game/Blueprints/BP_Dog.BP_Dog_C|GetInteger _dog_ai))
  (Variables|Default|SetMisson%20Objects (Variables|/Game/Blueprints/AIC_Companion.AIC_Companion_C|GetMissonObjects (Variables|/Game/Blueprints/BP_Dog.BP_Dog_C|GetAs%20AIC%20Companion _dog_ai))))