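; BP_JumpBlocks is a blocks actor that can test whether the moveable dumpster (BP_MoveableP) is near its Cube1 component.
; On BeginPlay it caches the first BP_MoveableP it finds as DumpsterRef.
; DistanceCheck returns true when that actor is within a fixed range of Cube1, otherwise prints the distance and returns false.
; The DistanceCheck call in its own event graph is unconnected, so nothing here runs the test.
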(event EventBeginPlay
  (bind _returnvalue (Actor|GetActorOfClass "/Game/Blueprints/Puzzles/Moveables/BP_MoveableP.BP_MoveableP_C"))
  (Variables|Default|SetDumpsterRef _returnvalue))

(fn ConstructionScript)

(fn DistanceCheck
  (bind _dumpsterref (Variables|Default|GetDumpsterRef))
  (bind _cube1 (Variables|Default|GetCube1))
  (bind _returnvalue (Transformation|GetActorLocation _dumpsterref))
  (bind _returnvalue_2 (Transformation|GetWorldLocation _cube1))
  (bind _returnvalue_3 (Math|Vector|Distance(Vector) _returnvalue_2 _returnvalue))
  (if (<= _returnvalue_3 3e+02)
    (return true)
    (else
      (Development|PrintString (Utilities|String|ToString(Float) _returnvalue_3))
      (return false))))