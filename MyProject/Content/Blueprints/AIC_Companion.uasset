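; AIC_Companion is the companion dog's brain, choosing which point of interest the dog heads to.
; At BeginPlay it caches all BP_POI actors, the dog and the first-person character, then picks a POI one tick later.
; The lowest score wins, weighting distance to player over distance to dog, plus Trust and Fear offsets identical for every POI.
; The winning location goes to the dog's Follow, and RemovePOI drops that POI from the list.
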(event Custom|Get%20POI
  (Variables|Default|SetHighest%20POI%20Score 999999.0)
  (for (_array_element _array_index) (Variables|Default|GetPOI_Array)
    (bind _output_get (Variables|Default|SetCurrentPOIScore (+ (* (Math|Vector|Distance(Vector) (Transformation|GetActorLocation _array_element) (Transformation|GetActorLocation (Variables|Default|GetFirstPersonCharacter_Ref))) 0.5) (* (Math|Vector|Distance(Vector) (Transformation|GetActorLocation _array_element) (Transformation|GetActorLocation (Variables|Default|GetDogRef))) 0.3) (* (Variables|Default|GetTrust) 1e+01) (* (Variables|Default|GetFear) -1e+01))))
    (if (<= _output_get (Variables|Default|GetHighest%20POI%20Score))
      (Variables|Default|SetHighest%20POI%20Score (Variables|Default|GetCurrentPOIScore))
      (Variables|Default|SetPOIIndex _array_index)))
  (Default|Follow (Variables|Default|GetDogRef) (Transformation|GetActorLocation (Utilities|Array|Get(acopy) (Variables|Default|GetPOI_Array) (Variables|Default|GetPOIIndex)))))

(event Custom|Initilaise
  (bind _outactors (Actor|GetAllActorsOfClass "/Game/Blueprints/BP_POI.BP_POI_C"))
  (Variables|Default|SetPOI_Array _outactors)
  (bind _returnvalue (Actor|GetActorOfClass "/Game/Blueprints/BP_Dog.BP_Dog_C"))
  (Variables|Default|SetDogRef _returnvalue)
  (bind _returnvalue_2 (Actor|GetActorOfClass "/Game/FirstPerson/Blueprints/BP_FirstPersonCharacter.BP_FirstPersonCharacter_C"))
  (bind _output_get (Variables|Default|SetFirstPersonCharacter_Ref _returnvalue_2))
  (Default|Initialise _output_get (Variables|Default|GetDogRef))
  (Utilities|FlowControl|DelayUntilNextTick)
  (CallFunction|GetPOI))

(event Custom|RemovePOI
  (bind _poi_array (Variables|Default|GetPOI_Array))
  (Utilities|Array|RemoveItem _poi_array (Utilities|Array|Get(acopy) _poi_array (Variables|Default|GetPOIIndex))))

(event Custom|CustomEvent)

(event EventBeginPlay
  (CallFunction|Initilaise))

(fn ConstructionScript)