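; BP_ProgressionPoint is a level-end trigger that ends the current level when the first-person player character walks into it.
; Shortly after BeginPlay it caches the ProgressManager from BP_CustomGameInstance.
; An overlap on its Box by exactly BP_FirstPersonCharacter calls EndLevel on that manager after a short delay.
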(event OnComponentBeginOverlap(Box)
  (params (OverlappedComponent :type Primitive%20Component%20Object%20Reference) (OtherActor :type Actor%20Object%20Reference) (OtherComp :type Primitive%20Component%20Object%20Reference) (OtherBodyIndex :type Integer) (bFromSweep :type Boolean) (SweepResult :type Hit%20Result%20Structure%20%28by%20ref%29))
  (if (== (Utilities|GetClass OtherActor) "/Game/FirstPerson/Blueprints/BP_FirstPersonCharacter.BP_FirstPersonCharacter_C")
    (Utilities|FlowControl|Delay 0.8)
    (Default|EndLevel (Variables|Default|GetProgress%20Manager))))

(event EventBeginPlay
  (Utilities|FlowControl|Delay 0.1)
  (bind _asbp_custom_game_instance (Utilities|Casting|CastToBP_CustomGameInstance (Game|GetGameInstance)))
  (Variables|Default|SetProgress%20Manager (Variables|/Game/Blueprints/Data/BP_CustomGameInstance.BP_CustomGameInstance_C|GetProgress%20Manager _asbp_custom_game_instance)))

(fn ConstructionScript)