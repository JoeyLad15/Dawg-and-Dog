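; BP_DogFoodPickUp is a puzzle pickup Blueprint, named for dog food, that defers to its parent class for its construction script and Tick.
; Each Tick, when PopUpText is not hidden in game, it rotates that text to face the player character's location using a look-at rotation.
; BeginPlay and overlap events are disabled stubs, and the graph holds no pickup logic of its own.
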(event EventBeginPlay
  (|CallParentFunction) ; This node is disabled and will not be called.\nDrag off pins to build functionality.
)

(event Collision|EventActorBeginOverlap
  (params (OtherActor :type Actor%20Object%20Reference))
  (|CallParentFunction OtherActor) ; This node is disabled and will not be called.\nDrag off pins to build functionality.
)

(event EventTick
  (params (DeltaSeconds :type Float%20%28single-precision%29))
  (bind _popuptext (Variables|Default|GetPopUpText))
  (|CallParentFunction DeltaSeconds)
  (if (not (Variables|/Script/Engine.SceneComponent|GetbHiddenInGame _popuptext))
    (Transformation|SetWorldRotation _popuptext (Math|Rotator|FindLookatRotation (Transformation|GetWorldLocation (Variables|Default|GetPopUpText)) (Transformation|GetActorLocation (Game|GetPlayerCharacter 0))) false false)))

(fn ConstructionScript
  (|CallParentFunction))