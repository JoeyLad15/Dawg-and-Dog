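; BP_BowlInteract is a puzzle interactable bowl that the player fills with dog food from their inventory.
; Interact checks TempInventory for DogFood: if found, it shows StaticMesh1, sets IsFilled, calls the player's Whistle, clears the prompt and removes one item; otherwise the prompt says food is needed.
; InteractionComplete hides the mesh again before calling the parent.
; Tick turns the visible pop-up text toward the player.
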(event EventBeginPlay
  (|CallParentFunction))

(event EventTick
  (params (DeltaSeconds :type Float%20%28single-precision%29))
  (bind _popuptext (Variables|Default|GetPopUpText))
  (|CallParentFunction DeltaSeconds)
  (if (not (Variables|/Script/Engine.SceneComponent|GetbHiddenInGame _popuptext))
    (Transformation|SetWorldRotation _popuptext (Math|Rotator|FindLookatRotation (Transformation|GetWorldLocation (Variables|Default|GetPopUpText)) (Transformation|GetActorLocation (Game|GetPlayerCharacter 0))) false false)))

(event EventInteract
  (if (.ReturnValue (Utilities|Map|Find (Variables|/Game/FirstPerson/Blueprints/BP_FirstPersonCharacter.BP_FirstPersonCharacter_C|GetTempInventory (Variables|Default|GetPlayer%20Ref)) "DogFood"))
    (Development|SetHiddeninGame (Variables|Default|GetStaticMesh1) false false)
    (Variables|Default|SetIsFilled? true)
    (Default|Whistle (Variables|Default|GetPlayer%20Ref))
    (bind _output_get (Variables|Default|SetCustomText ""))
    (Rendering|Components|TextRender|SetText (Variables|Default|GetPopUpText) _output_get)
    (Default|RemovefromInventory (Variables|Default|GetPlayer%20Ref) "DogFood" 1)
    (else
      (bind _output_get_2 (Variables|Default|SetCustomText "You Need Dog Food"))
      (Rendering|Components|TextRender|SetText (Variables|Default|GetPopUpText) _output_get_2))))

(event EventInteractionComplete
  (Development|SetHiddeninGame (Variables|Default|GetStaticMesh1) true false)
  (|CallParentFunction))

(fn ConstructionScript
  (|CallParentFunction))