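; BP_Door is a puzzle door actor that swings its static mesh open on Interact and back on CloseDoor.
; Each event plays its own timeline, lerping relative yaw toward a fixed open or closed angle while keeping pitch and roll.
; The lerp starts from the current rotation each update with a scaled-down alpha, giving an eased approach.
; A delayed auto-close is left unconnected, so nothing here calls CloseDoor.
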(event Custom|CloseDoor
  (bind _staticmesh (Variables|Default|GetStaticMesh))
  (bind _relativerotation (Variables|/Script/Engine.SceneComponent|GetRelativeRotation _staticmesh))
  (bind _newtrack_0 (Timeline|Timeline_0 PlayFromStart)
    (:Update
      (Transformation|SetRelativeRotation (Variables|Default|GetStaticMesh) (Math|Rotator|Lerp(Rotator) (Variables|/Script/Engine.SceneComponent|GetRelativeRotation _staticmesh) (Math|Rotator|MakeRotator (.roll _relativerotation) (.pitch _relativerotation) -9e+01) (* _newtrack_0 0.3) true) false false))))

(event EventBeginPlay
  (|CallParentFunction) ; This node is disabled and will not be called.\nDrag off pins to build functionality.
)

(event Collision|EventActorBeginOverlap
  (params (OtherActor :type Actor%20Object%20Reference))
  (|CallParentFunction OtherActor) ; This node is disabled and will not be called.\nDrag off pins to build functionality.
)

(event EventTick
  (params (DeltaSeconds :type Float%20%28single-precision%29))
  (|CallParentFunction DeltaSeconds) ; This node is disabled and will not be called.\nDrag off pins to build functionality.
)

(event EventInteract
  (bind _staticmesh (Variables|Default|GetStaticMesh))
  (bind _relativerotation (Variables|/Script/Engine.SceneComponent|GetRelativeRotation _staticmesh))
  (bind _newtrack_0 (Timeline|Timeline PlayFromStart)
    (:Update
      (Transformation|SetRelativeRotation (Variables|Default|GetStaticMesh) (Math|Rotator|Lerp(Rotator) (Variables|/Script/Engine.SceneComponent|GetRelativeRotation _staticmesh) (Math|Rotator|MakeRotator (.roll _relativerotation) (.pitch _relativerotation) 6e+01) (* _newtrack_0 0.3) true) false false))))

(fn ConstructionScript)