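; BP_LockedDoor is a puzzle door that the player unlocks with a Basement Key.
; Its Interact event looks up the key in the player's TempInventory and removes one if present.
; It then disables collision on the static mesh, without moving it, and sets the pop-up text to show the unlocked state.
; The key name is hardcoded, and nothing happens when the key is missing.
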(event EventBeginPlay
  (|CallParentFunction) ; This node is disabled and will not be called.\nDrag off pins to build functionality.
)

(event Collision|EventActorBeginOverlap
  (params (OtherActor :type Actor%20Object%20Reference))
  (|CallParentFunction OtherActor) ; This node is disabled and will not be called.\nDrag off pins to build functionality.
)

(event EventTick
  (params (DeltaSeconds :type Float%20%28single-precision%29))
  (|CallParentFunction DeltaSeconds) ; This node is disabled and will not be called.\nDrag off pins to build functionality.
)

(event EventInteract
  (if (> (.Value (Utilities|Map|Find (Variables|/Game/FirstPerson/Blueprints/BP_FirstPersonCharacter.BP_FirstPersonCharacter_C|GetTempInventory (Variables|Default|GetPlayer%20Ref)) "Basement Key")) 0)
    (Default|RemovefromInventory (Variables|Default|GetPlayer%20Ref) "Basement Key" 1)
    (Collision|SetCollisionEnabled (Variables|Default|GetStaticMesh) "NoCollision")
    (Rendering|Components|TextRender|SetText (Variables|Default|GetPopUpText) (Variables|Default|GetUnlocked))))

(fn ConstructionScript
  (|CallParentFunction))