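; Locked puzzle door Blueprint that swings open when the player interacts with it while carrying a Basement Key.
; Interact checks the player's TempInventory for the key, removes one and plays a timeline from the start.
; Each timeline update lerps the static mesh's yaw from its current rotation toward a fixed open angle, using the scaled track value as alpha.
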(event EventBeginPlay
  (|CallParentFunction) ; This node is disabled and will not be called.\nDrag off pins to build functionality.
)

(event Collision|EventActorBeginOverlap
  (params (OtherActor :type Actor%20Object%20Reference))
  (|CallParentFunction OtherActor) ; This node is disabled and will not be called.\nDrag off pins to build functionality.
)

(event EventTick
  (params (DeltaSeconds :type Float%20%28single-precision%29))
  (|CallParentFunction DeltaSeconds) ; This node is disabled and will not be called.\nDrag off pins to build functionality.
)

(event EventInteract
  (bind _staticmesh (Variables|Default|GetStaticMesh))
  (bind _relativerotation (Variables|/Script/Engine.SceneComponent|GetRelativeRotation _staticmesh))
  (if (> (.Value (Utilities|Map|Find (Variables|/Game/FirstPerson/Blueprints/BP_FirstPersonCharacter.BP_FirstPersonCharacter_C|GetTempInventory (Variables|Default|GetPlayer%20Ref)) "Basement Key")) 0)
    (Default|RemovefromInventory (Variables|Default|GetPlayer%20Ref) "Basement Key" 1)
    (bind _newtrack_0 (Timeline|Timeline_1 PlayFromStart)
      (:Update
        (Transformation|SetRelativeRotation (Variables|Default|GetStaticMesh) (Math|Rotator|Lerp(Rotator) (Variables|/Script/Engine.SceneComponent|GetRelativeRotation _staticmesh) (Math|Rotator|MakeRotator (.roll _relativerotation) (.pitch _relativerotation) 5e+01) (* _newtrack_0 0.3) true) false false)))))

(fn ConstructionScript
  (|CallParentFunction))